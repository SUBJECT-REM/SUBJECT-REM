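; Base interactable that stays gated until a matching key is used, with empty open and close functions as stubs.
; UseKey compares the item ID to the required key name, enables interaction, and also unlocks a linked actor if one is valid.
; Only with a valid link do both indicator widgets switch to the open-key image.
; Pressing interact stores the interactor and calls Open once interaction is enabled.
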(event EventBeginPlay)

(event Collision|EventActorBeginOverlap
  (params (OtherActor :type Actor%20Object%20Reference)))

(event EventTick
  (params (DeltaSeconds :type Float%20%28single-precision%29)))

(event EventUseKey
  (params (ItemId :type Name :default "None") (InstigatorActor :type Actor%20Object%20Reference))
  (bind _linkedactor (Variables|Default|GetLinkedActor))
  (bind _output (Utilities|ResolveSoftReference _linkedactor))
  (if (CallFunction|CanUseKey ItemId)
    (Variables|Default|SetCanUseInteract true)
    (Utilities|IsValid _output
      (:Is%20Valid
        (Variables|BP_InteractableWithKey_C|SetCanUseInteract _output true)
        (Default|SetWidgetImage (Variables|Default|GetBP_SRInteractionIndicatorWidgetComp) "/Game/ART_Resource/UI/HUD/HUD_TR_Key_Open_A01.HUD_TR_Key_Open_A01")
        (Default|SetWidgetImage (Actor|GetComponentbyClass (Utilities|ResolveSoftReference (Variables|Default|GetLinkedActor)) "/Game/Blueprint/Interactable/BP_SRInteractionIndicatorWidgetComp.BP_SRInteractionIndicatorWidgetComp_C") "/Game/ART_Resource/UI/HUD/HUD_TR_Key_Open_A01.HUD_TR_Key_Open_A01")))))

(event EventInteractionPressed
  (params (Interactor :type Actor%20Object%20Reference))
  (Variables|Default|SetInteractor Interactor)
  (if (Variables|Default|GetCanUseInteract)
    (CallFunction|Open)))

(fn ConstructionScript)

(fn Open)

(fn Close)

(fn OpenIner)

(fn CloseIner)

(fn CanUseKey
  (params (ItemId :type Name :default "None"))
  (return (== ItemId (Variables|Default|GetRequireKeyName))))