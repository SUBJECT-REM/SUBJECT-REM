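; Interactable world pickup that, when interaction is released, plays sounds, hides itself and reports a completed objective to the game flow manager.
; A valid data table handler supplies the row used to build an SRItem for the interactor's inventory; without a table, only the hide and notify run.
; BeginPlay and OnLoaded use state flags to set collision, physics or visibility.
; The BP_GameFlowManager reference is looked up lazily and cached.
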(event EventBeginPlay
  (bind _usegravity (Variables|Default|GetUsegravity))
  (if (Variables|Rendering|GetbHidden)
    (Collision|SetCollisionEnabled (Variables|Default|GetBox) "NoCollision")
    (if _usegravity
      (Physics|SetSimulatePhysics (Variables|Default|GetStaticMesh) _usegravity)
      (if (not (Variables|Default|GetbActivate)) :!label _label
        (Collision|SetCollisionEnabled (Variables|Default|GetBox) "NoCollision")))
    (else
      (goto _label))))

(event Collision|EventActorBeginOverlap
  (params (OtherActor :type Actor%20Object%20Reference)))

(event EventTick
  (params (DeltaSeconds :type Float%20%28single-precision%29)))

(event EventInteractionReleased
  (params (Interactor :type Actor%20Object%20Reference))
  (bind _datatablehandler (Variables|Default|GetDataTableHandler))
  (bind _box (Variables|Default|GetBox))
  (bind _box_2 (Variables|Default|GetBox))
  (bind (_datatable _rowname) (Utilities|Struct|BreakDataTableRowHandle _datatablehandler))
  (if (Utilities|IsValid (Variables|Default|GetNewVar))
    (Audio|PlaySound2D (Variables|Default|GetNewVar) 1.0 1.0 0.0 0 0))
  (Utilities|IsValid _datatable
    (:Is%20Valid
      (bind _returnvalue (Utilities|GetDataTableRow _datatable _rowname)
        (:then
          (bind _output_get (Variables|Default|SetOut%20Row _returnvalue))
          (Audio|PlaySound2D (.pickupsound (.BaseInfo (Utilities|Struct|BreakSRItemData _output_get))) 1.0 1.0 0.0 0 0)
          (Variables|Default|SetInvenComp (Actor|GetComponentbyClass Interactor "/Script/Subject_Rem.SRInventoryComponent"))
          (bind _returnvalue_2 (Game|ConstructObjectfromClass "/Script/Subject_Rem.SRItem"))
          (Variables|Default|SetItem _returnvalue_2)
          (Class|SRItem|SetItemData _returnvalue_2 (Variables|Default|GetOut%20Row))
          (Class|SRInventoryComponent|AddItem (Variables|Default|GetInvenComp) (Variables|Default|GetItem))
          (Rendering|SetActorHiddenInGame true)
          (Variables|/Script/Engine.PrimitiveComponent|SetbGenerateOverlapEvents _box false)
          (Collision|SetCollisionEnabled _box "NoCollision")
          (Class|SRGameFlowManager|NotifyObjectiveCompleted (CallFunction|GetTutorialManager) (Variables|Default|GetNotifyObjectiveTag)))))
    (:Is%20Not%20Valid
      (Rendering|SetActorHiddenInGame true)
      (Variables|/Script/Engine.PrimitiveComponent|SetbGenerateOverlapEvents _box_2 false)
      (Collision|SetCollisionEnabled _box_2 "NoCollision")
      (Class|SRGameFlowManager|NotifyObjectiveCompleted (CallFunction|GetTutorialManager) (Variables|Default|GetNotifyObjectiveTag)))))

(event EventOnLoaded
  (if (not (Variables|Default|GetbActivate))
    (Rendering|SetActorHiddenInGame true)
    (Collision|SetCollisionEnabled (Variables|Default|GetBP_SRInteractionIndicatorWidgetComp) "NoCollision")
    (Collision|SetCollisionEnabled (Variables|Default|GetBox) "NoCollision")
    (Development|PrintString "Activate false ")))

(fn ConstructionScript)

(fn GetTutorialManager
  (Utilities|IsValid (Variables|Default|GetTutorialManager)
    (:Is%20Valid
      (return (stale _output_get)))
    (:Is%20Not%20Valid
      (bind _returnvalue (Actor|GetActorOfClass "/Game/Blueprint/ManagerActor/BP_GameFlowManager.BP_GameFlowManager_C"))
      (bind _output_get (Variables|Default|SetTutorialManager _returnvalue))
      (if (Utilities|IsValid _output_get)
        (return _output_get)))))