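; Interactable elevator that teleports the player to a linked elevator behind a screen fade.
; Opening plays a ding, opens the linked elevator and runs chained timelines sliding the lower then upper door body, before starting WBP_FadeInOut.
; Fade-in completion triggers the teleport, and CloseElevatorBoth reverses the doors at both ends and clears fade bindings.
; Completing Chapter 3 in BP_GameFlowManager switches destination to the override location and linked actor, when set.
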(event Custom|OpenElevatorOnlyAction
  (bind _downbodyorginloc (Variables|Default|GetDownBodyOrginLoc))
  (bind _upbodyoriginloc (Variables|Default|GetUpBodyOriginLoc))
  (bind (_x _y) (Math|Vector|BreakVector _downbodyorginloc))
  (bind (_x_2 _y_2 _z) (Math|Vector|BreakVector _upbodyoriginloc))
  ;[0.15 0.15 0.15 0.5] Elevator Open
  (bind _tl_bottom (Timeline|Timeline_3 PlayFromStart)
    (:Update
      (Transformation|SetRelativeLocation (Variables|Default|GetDownBody) (Math|Vector|Lerp(Vector) _downbodyorginloc (Math|Vector|MakeVector _x _y (Variables|Default|GetDownBodyOpenPos)) _tl_bottom) false false))
    (:Finished
      (bind _tl_top (Timeline|Timeline_4 PlayFromStart)
        (:Update
          (Transformation|SetWorldLocation (Variables|Default|GetUpBody) (Math|Vector|Lerp(Vector) _upbodyoriginloc (Math|Vector|MakeVector _x_2 _y_2 (+ _z (Variables|Default|GetUpBodyOpenPos))) _tl_top) false false))))))

(event Custom|OpenElevatorFadeInOut
  (bind _newparam (CallFunction|SelectLinkedActor))
  (bind _downbodyorginloc (Variables|Default|GetDownBodyOrginLoc))
  (bind _upbodyoriginloc (Variables|Default|GetUpBodyOriginLoc))
  (bind (_x _y _z) (Math|Vector|BreakVector _upbodyoriginloc))
  (bind (_x_2 _y_2) (Math|Vector|BreakVector _downbodyorginloc))
  (Audio|PlaySound2D "/Game/Audio/DoorSound/엘레베이터_띵동_.엘레베이터_띵동_" 1.0 1.0 0.0 0 0)
  (if (Utilities|IsValidSoftObjectReference _newparam)
    (CallFunction|OpenIner (Utilities|ResolveSoftReference _newparam))
    ;[0.15 0.15 0.15 0.5] Default 90
    (bind _tl_bottom (Timeline|Timeline PlayFromStart)
      (:Update
        (Transformation|SetRelativeLocation (Variables|Default|GetDownBody) (Math|Vector|Lerp(Vector) _downbodyorginloc (Math|Vector|MakeVector _x_2 _y_2 (Variables|Default|GetDownBodyOpenPos)) _tl_bottom) false false))
      (:Finished
        (bind _tl_top (Timeline|Timeline_0 PlayFromStart)
          (:Update
            (Transformation|SetWorldLocation (Variables|Default|GetUpBody) (Math|Vector|Lerp(Vector) _upbodyoriginloc (Math|Vector|MakeVector _x _y (+ _z (Variables|Default|GetUpBodyOpenPos))) _tl_top) false false))
          (:Finished
            (if (Utilities|IsValid (Variables|Default|GetFadeInOut))
              (if (UserInterface|Viewport|IsinViewport (Variables|Default|GetFadeInOut))
                (Default|PlayFadeinOut (Variables|Default|GetFadeInOut) (Variables|Default|GetDestinationIsBasementionOrGround) 0.0)
                (else
                  (UserInterface|Viewport|AddtoViewport (Variables|Default|GetFadeInOut) 0)
                  (Default|PlayFadeinOut (Variables|Default|GetFadeInOut) (Variables|Default|GetDestinationIsBasementionOrGround) 0.0)))
              (else
                (bind _returnvalue (UserInterface|CreateWidget "/Game/Blueprint/UI/HUD/Fade/WBP_FadeInOut.WBP_FadeInOut_C"))
                (UserInterface|Viewport|AddtoViewport _returnvalue 0)
                (Default|PlayFadeinOut _returnvalue (Variables|Default|GetDestinationIsBasementionOrGround) 0.0)))))))
    (else
      (Timeline|Timeline PlayFromStart))))

(event Custom|Teleport
  (bind _newparam (CallFunction|SelectLoc))
  (Development|PrintString (Utilities|String|ToString(Vector) _newparam))
  (Transformation|Teleport (Variables|Default|GetInteractor) _newparam (Variables|Default|GetTeleportRot)))

(event Custom|CloseElevatorOnlyAction
  (bind _upbodyoriginloc (Variables|Default|GetUpBodyOriginLoc))
  (bind _downbodyorginloc (Variables|Default|GetDownBodyOrginLoc))
  (bind (_x _y) (Math|Vector|BreakVector _downbodyorginloc))
  (bind (_x_2 _y_2 _z) (Math|Vector|BreakVector _upbodyoriginloc))
  ;[0.15 0.15 0.15 0.5] ElevatorMove
  (bind _tl_bottom (Timeline|Timeline_1 PlayFromStart)
    (:Update
      (Transformation|SetWorldLocation (Variables|Default|GetUpBody) (Math|Vector|Lerp(Vector) (Math|Vector|MakeVector _x_2 _y_2 (+ _z (Variables|Default|GetUpBodyOpenPos))) _upbodyoriginloc _tl_bottom) false false))
    (:Finished
      (bind _tl_top (Timeline|Timeline_2 PlayFromStart)
        (:Update
          (Transformation|SetRelativeLocation (Variables|Default|GetDownBody) (Math|Vector|Lerp(Vector) (Math|Vector|MakeVector _x _y (Variables|Default|GetDownBodyOpenPos)) _downbodyorginloc _tl_top) false false))))))

(event Custom|CloseElevatorBoth
  (bind _newparam (CallFunction|SelectLinkedActor))
  (bind _output (Utilities|ResolveSoftReference _newparam))
  (Utilities|IsValid _output
    (:Is%20Valid
      (CallFunction|Close _output))
    (:Is%20Not%20Valid
      _))
  (CallFunction|Close)
  (CallFunction|ClearFadeOut))

(event Custom|FlowComplete
  (params (CompleteId :type Gameplay%20Tag%20Structure))
  (if (== CompleteId "(TagName=\"GameFlow.Chapter3Complete\")")
    (if (and (Utilities|Operators|NotEqual(!=) (Variables|Default|GetOverrideLoc) (Math|Vector|VectorZero) 0.0) (Utilities|IsValidSoftObjectReference (Variables|Default|GetOverrideLinkedACtor)))
      (Variables|Default|SetDestinationIsBasementionOrGround true)
      (Development|PrintString "Chapter3 Comp")
      (else
        (Development|PrintString "Chapter3 Comp Not OverrideLoc")))))

(event EventBeginPlay
  (Variables|Default|SetDownBodyOrginLoc (Variables|/Script/Engine.SceneComponent|GetRelativeLocation (Variables|Default|GetDownBody)))
  (Variables|Default|SetUpBodyOriginLoc (Transformation|GetWorldLocation (Variables|Default|GetUpBody)))
  (bind _returnvalue (UserInterface|CreateWidget "/Game/Blueprint/UI/HUD/Fade/WBP_FadeInOut.WBP_FadeInOut_C"))
  (Variables|Default|SetFadeInOut _returnvalue)
  (bind _returnvalue_2 (Actor|GetActorOfClass "/Game/Blueprint/ManagerActor/BP_GameFlowManager.BP_GameFlowManager_C"))
  (Utilities|IsValid _returnvalue_2
    (:Is%20Valid
      (if (not (Math|Vector|VectorIsZero (Variables|Default|GetOverrideLoc)))
        (EventDispatchers|BindEventtoOnFlowCompleteDelegate _returnvalue_2 (EventDispatchers|CreateEvent :!event Custom|FlowComplete))))))

(event Collision|EventActorBeginOverlap
  (params (OtherActor :type Actor%20Object%20Reference)))

(event EventInteractionReleased
  (params (Interactor :type Actor%20Object%20Reference))
  (bind _asplayer_controller (Utilities|Casting|CastToPlayerController (Game|GetInstigatorController Interactor)))
  (bind _assr_hud (Utilities|Casting|CastToSR_HUD (HUD|GetHUD _asplayer_controller)))
  (Utilities|IsValid (Class|SRHUD|GetWidgetbyClass _assr_hud "/Game/Blueprint/UI/HUD/Fade/WBP_FadeInOut.WBP_FadeInOut_C" true)
    (:Is%20Valid
      (bind _output_get (Variables|Default|SetFadeInOut (Class|SRHUD|GetWidgetbyClass _assr_hud "/Game/Blueprint/UI/HUD/Fade/WBP_FadeInOut.WBP_FadeInOut_C" true)))
      (EventDispatchers|BindEventtoFadeinFinish _output_get (delegate Custom|Teleport))
      (EventDispatchers|BindEventtoFadeOutFinish _output_get (EventDispatchers|CreateEvent :!event Custom|CloseElevatorBoth)))))

(fn ConstructionScript)

(fn Open
  (|CallParentFunction)
  (CallFunction|OpenElevatorFadeinOut))

(fn OpenIner
  (|CallParentFunction)
  (CallFunction|OpenElevatorOnlyAction))

(fn Close
  (|CallParentFunction)
  (CallFunction|CloseElevatorOnlyAction))

(fn SelectLoc
  (if (and (Variables|Default|GetDestinationIsBasementionOrGround) (Utilities|Operators|NotEqual(!=) (Variables|Default|GetOverrideLoc) (Math|Vector|VectorZero) 0.0))
    (return (Variables|Default|GetOverrideLoc))
    (else
      (return (Variables|Default|GetTeleportLoc)))))

(fn SelectLinkedActor
  (if (Variables|Default|GetDestinationIsBasementionOrGround)
    (return (Variables|Default|GetOverrideLinkedACtor))
    (else
      (return (Variables|Default|GetLinkedActor)))))

(fn ClearFadeOut
  (EventDispatchers|UnbindEventfromFadeinFinish (Variables|Default|GetFadeInOut) (EventDispatchers|CreateEvent :!event Custom|Teleport))
  (EventDispatchers|UnbindEventfromFadeOutFinish (Variables|Default|GetFadeInOut) (EventDispatchers|CreateEvent :!event Custom|CloseElevatorBoth))
  (Variables|Default|SetFadeInOut 0))