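; Presenter Blueprint that links clue data in the inventory component to the clue UI widget.
; Init calls the parent, then casts and caches the BP_InventoryComp and WB_Clue it receives, binding an event to the component's AddClueData delegate.
; UpdateClueView forwards its parameter to the widget's UpdateClue, keeping the component and widget decoupled in a Model-View-Presenter style.
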(fn Init
  (params (InitComponent :type BP%20Inventory%20Comp%20Object%20Reference) (Init%20Widget :type User%20Widget%20Object%20Reference))
  (|CallParentFunction InitComponent Init%20Widget)
  (Utilities|FlowControl|Sequence
    (:then_0
      (bind _asbp_inventory_comp (Utilities|Casting|CastToBP_InventoryComp InitComponent))
      (bind _output_get (Variables|Default|SetInventoryComp _asbp_inventory_comp))
      (EventDispatchers|BindEventtoAddClueDataDelegate _asbp_inventory_comp (EventDispatchers|CreateEvent :!event UpdateClueView)))
    (:then_1
      (bind _aswb_clue (Utilities|Casting|CastToWB_Clue Init%20Widget))
      (Variables|Default|SetClueWidget _aswb_clue))))

(fn UpdateClueView
  (params (NewParam :type ST%20Clue%20Data%20Structure))
  (Default|UpdateClue (Variables|Default|GetClueWidget) NewParam))