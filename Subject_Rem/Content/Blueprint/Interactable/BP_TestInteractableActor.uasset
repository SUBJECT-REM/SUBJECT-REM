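; Test interactable pickup actor that gives its item to the interacting actor's inventory.
; On interaction release, it looks up its data table row, builds an SRItem from that data and adds it to the interactor's SRInventoryComponent.
; It then hides itself and disables the Box's overlap events and collision rather than being destroyed; nothing happens if the row is not found.
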(event EventBeginPlay)

(event Collision|EventActorBeginOverlap
  (params (OtherActor :type Actor%20Object%20Reference)))

(event EventTick
  (params (DeltaSeconds :type Float%20%28single-precision%29)))

(event EventInteractionReleased
  (params (Interactor :type Actor%20Object%20Reference))
  (bind _datatablehandler (Variables|Default|GetDataTableHandler))
  (bind _box (Variables|Default|GetBox))
  (bind (_datatable _rowname) (Utilities|Struct|BreakDataTableRowHandle _datatablehandler))
  (bind _returnvalue (Utilities|GetDataTableRow _datatable _rowname)
    (:then
      (bind _returnvalue_2 (Game|ConstructObjectfromClass "/Script/Subject_Rem.SRItem"))
      (Class|SRItem|SetItemData _returnvalue_2 _returnvalue)
      (Class|SRInventoryComponent|AddItem (Actor|GetComponentbyClass Interactor "/Script/Subject_Rem.SRInventoryComponent") _returnvalue_2)
      (Rendering|SetActorHiddenInGame true)
      (Variables|/Script/Engine.PrimitiveComponent|SetbGenerateOverlapEvents _box false)
      (Collision|SetCollisionEnabled _box "NoCollision"))))

(fn ConstructionScript)