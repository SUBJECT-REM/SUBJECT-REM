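; BP_Window is an interactable window that swings open and teleports the interactor behind a screen fade, working as a pair with a linked actor.
; Timelines lerp the window between its initial rotation and one built from an open angle.
; Opening also opens the linked actor, then plays the fade widget, whose fade-in callback performs the teleport.
; Inner open/close overrides move only this window, and a cabinet sound accompanies opening and closing.
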(event Custom|OpenWindow
  (Development|PrintString (Utilities|String|ToString(Rotator) (Variables|Default|GetOriginActorRot)))
  (bind _open (Timeline|Timeline_1 PlayFromStart)
    (:Update
      (Transformation|SetRelativeRotation (Variables|Default|GetWindow) (Math|Rotator|Lerp(Rotator) (Variables|Default|GetOriginActorRot) (Variables|Default|GetOpenWindowRot) _open) false false))))

(event Custom|CloseWindow
  (Development|PrintString (Utilities|String|ToString(Rotator) (Variables|Default|GetOpenWindowRot)))
  (bind _newtrack_0 (Timeline|Timeline_0 PlayFromStart)
    (:Update
      (Transformation|SetRelativeRotation (Variables|Default|GetWindow) (Math|Rotator|Lerp(Rotator) (Variables|Default|GetOpenWindowRot) (Variables|Default|GetOriginActorRot) _newtrack_0) false false))
    (:Finished
      (Audio|PlaySound2D "/Game/Audio/InteractionSound/상호작용_캐비넷_.상호작용_캐비넷_" 1.0 1.0 0.0 0 0))))

(event Custom|CustomEvent
  (Transformation|Teleport (Variables|Default|GetInteractor) (Variables|Default|GetTeleportLoc) (Variables|Default|GetTeleportRot)))

(event Custom|OpenWindowWithFadeIn
  (CallFunction|OpenIner (Utilities|ResolveSoftReference (Variables|Default|GetLinkedActor)))
  (bind _open (Timeline|Timeline PlayFromStart)
    (:Update
      (Transformation|SetRelativeRotation (Variables|Default|GetWindow) (Math|Rotator|Lerp(Rotator) (Variables|Default|GetOriginActorRot) (Variables|Default|GetOpenWindowRot) _open) false false))
    (:Finished
      (if (Utilities|IsValid (Variables|Default|GetFadeInOut))
        (if (UserInterface|Viewport|IsinViewport (Variables|Default|GetFadeInOut))
          (Default|PlayFadeinOut (Variables|Default|GetFadeInOut))
          (else
            (UserInterface|Viewport|AddtoViewport (Variables|Default|GetFadeInOut) 0)
            (Default|PlayFadeinOut (Variables|Default|GetFadeInOut))))
        (else
          (bind _returnvalue (UserInterface|CreateWidget "/Game/Blueprint/UI/HUD/Fade/WBP_FadeInOut.WBP_FadeInOut_C"))
          (UserInterface|Viewport|AddtoViewport _returnvalue 0)
          (Default|PlayFadeinOut _returnvalue))))))

(event Custom|CloseWindowBoth
  (CallFunction|CloseIner (Utilities|ResolveSoftReference (Variables|Default|GetLinkedActor)))
  (CallFunction|Close))

(event EventBeginPlay
  (bind _output_get (Variables|Default|SetOriginActorRot (Variables|/Script/Engine.SceneComponent|GetRelativeRotation (Variables|Default|GetWindow))))
  ;[0.15 0.15 0.15 0.5] Default 90
  (bind _output_get_2 (Variables|Default|SetOpenWindowRot (Math|Rotator|MakeRotator (Variables|Default|GetOpenDegre) (.pitch _output_get) (.yaw _output_get))))
  (bind _returnvalue (UserInterface|CreateWidget "/Game/Blueprint/UI/HUD/Fade/WBP_FadeInOut.WBP_FadeInOut_C"))
  (bind _output_get_3 (Variables|Default|SetFadeInOut _returnvalue))
  (EventDispatchers|BindEventtoFadeinFinish _output_get_3 (delegate Custom|CustomEvent))
  (EventDispatchers|BindEventtoFadeOutFinish _output_get_3 (EventDispatchers|CreateEvent :!event Custom|CloseWindowBoth)))

(event Collision|EventActorBeginOverlap
  (params (OtherActor :type Actor%20Object%20Reference)))

(fn ConstructionScript)

(fn Open
  (|CallParentFunction)
  (CallFunction|OpenWindowwithFadein)
  (Audio|PlaySound2D "/Game/Audio/InteractionSound/상호작용_캐비넷_.상호작용_캐비넷_" 1.0 1.0 0.0 0 0))

(fn Close
  (|CallParentFunction)
  (CallFunction|CloseWindow))

(fn OpenIner
  (|CallParentFunction)
  (CallFunction|OpenWindow))

(fn CloseIner
  (|CallParentFunction)
  (CallFunction|CloseWindow))