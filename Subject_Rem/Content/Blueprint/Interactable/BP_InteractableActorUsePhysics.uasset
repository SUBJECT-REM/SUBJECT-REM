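; Interactable actor Blueprint for a physics-driven object that settles on impact, with a key-drop sound (열쇠_떨어짐).
; On a static mesh hit it prints the other actor's name, shows the Niagara effect, turns off physics simulation and plays the sound in 2D.
; The hit handler has no filter on the other actor or guard against repeats, and EnableEffectAfterOnHit is unused.
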(event OnComponentHit(StaticMesh)
  (params (HitComponent :type Primitive%20Component%20Object%20Reference) (OtherActor :type Actor%20Object%20Reference) (OtherComp :type Primitive%20Component%20Object%20Reference) (NormalImpulse :type Vector :default "0, 0, 0") (Hit :type Hit%20Result%20Structure%20%28by%20ref%29))
  (Development|PrintString (Utilities|String|Append "OnHit  : " (Utilities|GetDisplayName OtherActor)))
  (Rendering|SetVisibility (Variables|Default|GetNiagara) true false)
  (Physics|SetSimulatePhysics (Variables|Default|GetStaticMesh) false)
  (Audio|PlaySound2D "/Game/Audio/열쇠_떨어짐.열쇠_떨어짐" 1.0 1.0 0.0 0 0))

(event EventBeginPlay
  (|CallParentFunction))

(event Collision|EventActorBeginOverlap
  (params (OtherActor :type Actor%20Object%20Reference))
  (|CallParentFunction OtherActor) ; This node is disabled and will not be called.\nDrag off pins to build functionality.
)

(event EventTick
  (params (DeltaSeconds :type Float%20%28single-precision%29))
  (|CallParentFunction DeltaSeconds) ; This node is disabled and will not be called.\nDrag off pins to build functionality.
)

(fn ConstructionScript
  (|CallParentFunction))