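; Interactable sliding door that automatically walks the player to a front or back point, with player input restricted during the sequence.
; Interaction starts a Tick-driven, flag-based sequence: lerp the Cube open, pause, move the character, then lerp it closed and restore input.
; Front and back overlap boxes choose the destination.
; SimpleMoveToLocation drives the walk while side-scroller AnimBP variables are forced, and X-distance detects arrival.
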(event OnComponentBeginOverlap(BackBox)
  (params (OverlappedComponent :type Primitive%20Component%20Object%20Reference) (OtherActor :type Actor%20Object%20Reference) (OtherComp :type Primitive%20Component%20Object%20Reference) (OtherBodyIndex :type Integer) (bFromSweep :type Boolean) (SweepResult :type Hit%20Result%20Structure%20%28by%20ref%29))
  (Variables|Default|SetbIsOverlapingFront false))

(event OnComponentBeginOverlap(FrontBox)
  (params (OverlappedComponent :type Primitive%20Component%20Object%20Reference) (OtherActor :type Actor%20Object%20Reference) (OtherComp :type Primitive%20Component%20Object%20Reference) (OtherBodyIndex :type Integer) (bFromSweep :type Boolean) (SweepResult :type Hit%20Result%20Structure%20%28by%20ref%29))
  (Variables|Default|SetbIsOverlapingFront true)
  (Development|PrintString "Overlap Front"))

(event OnComponentEndOverlap(FrontBox)
  (params (OverlappedComponent :type Primitive%20Component%20Object%20Reference) (OtherActor :type Actor%20Object%20Reference) (OtherComp :type Primitive%20Component%20Object%20Reference) (OtherBodyIndex :type Integer))
  (Variables|Default|SetbIsOverlapingFront false))

(event Custom|MoveToPosition
  (if (Variables|Default|GetbIsOverlapingFrontChach)
    (if (< (Math|Float|Absolute(Float) (- (.x (Transformation|GetWorldLocation (Variables|/Script/Engine.Actor|GetRootComponent (Game|Player|GetPlayerPawn 0)))) (.x (Transformation|GetWorldLocation (Variables|Default|GetFrontMovePosition))))) 5e+01)
      (Variables|Default|SetbIsOverlapMoveing false :!label _label)
      (Variables|Default|SetbIsDoorClose true)
      (Variables|Default|SetDoorOpenCloseAlpha 0.0))
    (elif (< (Math|Float|Absolute(Float) (- (.x (Transformation|GetWorldLocation (Variables|/Script/Engine.Actor|GetRootComponent (Game|Player|GetPlayerPawn 0)))) (.x (Transformation|GetWorldLocation (Variables|Default|GetBackMovePosition))))) 5e+01)
      (goto _label))))

(event Custom|DoorOpen
  (params (DeltaTime :type Float%20%28double-precision%29))
  ;[0.15 0.15 0.15 0.5] Door Moving
  ;;[0.15 0.15 0.15 0.5] DeltaTime을 이용하여 Lerp로 문을 이동시킵니다.
  (bind _output_get (Variables|Default|SetDoorOpenCloseAlpha (+ DeltaTime (Variables|Default|GetDoorOpenCloseAlpha))))
  (if (<= _output_get 1.0)
    (Transformation|SetWorldLocation (Variables|Default|GetCube) (Math|Vector|Lerp(Vector) (Variables|Default|GetOriginWorldLocation) (Variables|Default|GetOpenWorldLocation) _output_get) false false)
    (else
      ;;[0.15 0.15 0.15 0.5] 문이 다 열리고 이동합니다.
      (Utilities|FlowControl|Delay 0.5)
      (Variables|Default|SetbIsDoorOpen false)
      (Variables|Default|SetbIsOverlapMoveing true)
      (CallFunction|MoveCharacter))))

(event Custom|Move%20Character
  (bind _returnvalue (Game|Player|GetPlayerPawn 0))
  (bind _returnvalue_2 (Game|Player|GetPlayerPawn 0))
  (bind _frontmoveposition (Variables|Default|GetFrontMovePosition))
  (bind _backmoveposition (Variables|Default|GetBackMovePosition))
  (bind _returnvalue_3 (Transformation|GetWorldLocation _frontmoveposition))
  (bind _returnvalue_4 (Transformation|GetWorldLocation _backmoveposition))
  (if (Variables|Default|GetbIsOverlapingFrontChach)
    ;[0.15 0.15 0.15 0.5] FrontMovePosition으로 이동합니다.
    (AI|Navigation|SimpleMovetoLocation (Game|GetPlayerController 0) _returnvalue_3)
    (Transformation|SetActorRotation _returnvalue (Math|Rotator|FindLookatRotation (Transformation|GetActorLocation _returnvalue) _returnvalue_3))
    (else
      ;[0.15 0.15 0.15 0.5] BackMovePosition으로 이동합니다.
      (AI|Navigation|SimpleMovetoLocation (Game|GetPlayerController 0) _returnvalue_4)
      (Transformation|SetActorRotation _returnvalue_2 (Math|Rotator|FindLookatRotation (Transformation|GetActorLocation _returnvalue_2) _returnvalue_4)))))

(event Custom|DoorClose
  (params (DeltaTime :type Float%20%28double-precision%29))
  ;[0.15 0.15 0.15 0.5] Door Moving
  ;;[0.15 0.15 0.15 0.5] DeltaTime을 이용하여 Lerp로 문을 이동시킵니다.
  (bind _output_get (Variables|Default|SetDoorOpenCloseAlpha (+ DeltaTime (Variables|Default|GetDoorOpenCloseAlpha))))
  (if (<= _output_get 1.0)
    (Transformation|SetWorldLocation (Variables|Default|GetCube) (Math|Vector|Lerp(Vector) (Variables|Default|GetOpenWorldLocation) (Variables|Default|GetOriginWorldLocation) _output_get) false false)
    (else
      ;;[0.15 0.15 0.15 0.5] 문이 다 닫히고 Block을 해제하는 동작이 들어가야합니다.
      (Development|PrintString "Block Off")
      (Variables|Default|SetbIsDoorClose false)
      (Class|SRInputLocalPlayerSubsystem|RemoveInputRestriction (Subsystems|GetSRInputLocalPlayerSubsystem)))))

(event EventBeginPlay
  (bind _ascharacter (Utilities|Casting|CastToCharacter (Game|Player|GetPlayerPawn 0)))
  (bind _asabp_manny_side_scroller (Utilities|Casting|CastToABP_Manny_SideScroller (Components|SkeletalMesh|GetAnimInstance (Variables|/Script/Engine.Character|GetMesh _ascharacter))))
  (Variables|Default|SetAs%20ABP%20Manny%20Side%20Scroller _asabp_manny_side_scroller)
  (Variables|Default|SetOriginWorldLocation (Transformation|GetWorldLocation (Variables|Default|GetCube)))
  ;[0.15 0.15 0.15 0.5] Y을 조절해서 이동량을 바꾸면 됩니다.
  (Variables|Default|SetOpenWorldLocation (- (Transformation|GetWorldLocation (Variables|Default|GetCube)) "0.000000,1000.000000,0.000000")))

(event EventTick
  (params (DeltaSeconds :type Float%20%28single-precision%29))
  (bind _as_abp_manny_side_scroller (Variables|Default|GetAs%20ABP%20Manny%20Side%20Scroller))
  (Utilities|FlowControl|Sequence
    (:then_0
      ;[0.15 0.15 0.15 0.5] 문을 엽니다.
      (if (Variables|Default|GetbIsDoorOpen)
        (CallFunction|DoorOpen DeltaSeconds)))
    (:then_1
      ;[0.15 0.15 0.15 0.5] 캐릭터가 Animation을 재생하며 이동합니다.
      (if (Variables|Default|GetbIsOverlapMoveing)
        (Variables|/Game/Variant_SideScrolling/Anims/ABP_Manny_SideScroller.ABP_Manny_SideScroller_C|SetShouldMove _as_abp_manny_side_scroller true)
        (Variables|/Game/Variant_SideScrolling/Anims/ABP_Manny_SideScroller.ABP_Manny_SideScroller_C|SetGround%20Forward%20Percent _as_abp_manny_side_scroller 1.0)
        (CallFunction|MovetoPosition)))
    (:then_2
      ;[0.15 0.15 0.15 0.5] 문을 닫습니다.
      (if (Variables|Default|GetbIsDoorClose)
        (CallFunction|DoorClose DeltaSeconds)))))

(event EventInteractionPressed
  (params (Interactor :type Actor%20Object%20Reference))
  (Variables|Default|SetDoorOpenCloseAlpha 0.0)
  (Variables|Default|SetbIsDoorOpen true)
  (Variables|Default|SetbIsOverlapingFrontChach (Variables|Default|GetbIsOverlapingFront))
  (Development|PrintString "ShouldBlock")
  (Class|SRInputLocalPlayerSubsystem|ApplyInputRestriction (Subsystems|GetSRInputLocalPlayerSubsystem)))

(fn ConstructionScript)