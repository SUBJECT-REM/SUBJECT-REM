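; BP_MainCharacter is the player character, with left/right movement and a toggleable investigation menu.
; On BeginPlay it creates the hidden menu widget from its SRInventory and registers a key widget with SRTutorial.
; Movement input drives it along a fixed world axis, and the first move notifies the tutorial's Move objective.
; The inventory input toggles menu visibility together with the mouse cursor.
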(event Input|EnhancedActionEvents|EnhancedInputActionIA_OpenInven
  (params (ActionValue :type Boolean) (ElapsedSeconds :type Float%20%28double-precision%29) (TriggeredSeconds :type Float%20%28double-precision%29) (InputAction :type Input%20Action%20Object%20Reference :default "/Game/Defender/Inputs/DigitalBoolInputActions/IA_OpenInven.IA_OpenInven"))
  (:Started
    (CallFunction|OpenInvestigationMenu)))

(event Input|EnhancedActionEvents|EnhancedInputActionIA_MoveRight
  (params (ActionValue :type Float%20%28double-precision%29) (ElapsedSeconds :type Float%20%28double-precision%29) (TriggeredSeconds :type Float%20%28double-precision%29) (InputAction :type Input%20Action%20Object%20Reference :default "/Game/Defender/Inputs/AxisInputActions/IA_MoveRight.IA_MoveRight"))
  (:Triggered
    (Variables|Default|SetMoveForwardAxisValue ActionValue)
    (Pawn|Input|AddMovementInput (Math|Vector|GetForwardVector "0, 0, 0") (Variables|Default|GetMoveForwardAxisValue) false)
    (if (not (Variables|Default|GetFirstMovfe))
      (Class|SRTutorialComponent|NotifyTutorialObjective (Variables|Default|GetSRTutorial) "(TagName=\"Tutorial.Objectives.Move\")")
      (Variables|Default|SetFirstMovfe true)))
  (:Completed
    (Variables|Default|SetMoveForwardAxisValue 0.0)))

(event EventBeginPlay
  (CallFunction|CreateInvenstigationMenu)
  (Class|SRTutorialComponent|SetTutorialWidgetComponent (Variables|Default|GetSRTutorial) (Variables|Default|GetTutorialKeyWidget)))

(fn ConstructionScript)

(fn OpenInvestigationMenu
  (if (Variables|Default|GetIsInvestigationMenuOpen)
    (Widget|SetVisibility (Variables|Default|GetInvestigationMenu) "Hidden")
    (Variables|Default|SetIsInvestigationMenuOpen false)
    (Variables|/Script/Engine.PlayerController|SetbShowMouseCursor (Game|GetPlayerController 0) false)
    (else
      (Widget|SetVisibility (Variables|Default|GetInvestigationMenu) "Visible")
      (Variables|Default|SetIsInvestigationMenuOpen true)
      (Variables|/Script/Engine.PlayerController|SetbShowMouseCursor (Game|GetPlayerController 0) true))))

(fn CreateInvenstigationMenu
  (if (not (Utilities|IsValid (Variables|Default|GetInvestigationMenu)))
    (bind _returnvalue (UserInterface|CreateWidget "/Game/Blueprint/UI/Invenstigation/WB_InvestigationMenu.WB_InvestigationMenu_C"))
    (bind _output_get (Variables|Default|SetInvestigationMenu _returnvalue))
    (Class|SRInvestigationMenu|InitInvestigationMenuWidget _output_get (Variables|Default|GetSRInventory))
    (UserInterface|Viewport|AddtoViewport (Variables|Default|GetInvestigationMenu) 0)
    (Widget|SetVisibility (Variables|Default|GetInvestigationMenu) "Hidden")
    (Variables|Default|SetIsInvestigationMenuOpen false)))