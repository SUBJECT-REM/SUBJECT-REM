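; Caption manager actor that relays typewriter start and completion events from the game caption widget.
; Shortly after BeginPlay it caches the game flow manager and searches the SR_HUD's viewport widgets for WB_GameCaption to bind its typewriter events.
; Caption start and finish pass the row name to delegate calls, with finish also printing it.
; Tutorial pickup and actor activation logic remains in the graph but never runs.
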(event Custom|HandlePickupItemTuto
  (params (CompleteId :type Gameplay%20Tag%20Structure)))

(event Custom|OnCaptionStart
  (params (RowName :type Name))
  (Default|CallCaptionTypewriterStartDelgate RowName))

(event EventBeginPlay
  (bind _returnvalue (Game|GetPlayerController 0))
  (bind _returnvalue_2 (HUD|GetHUD _returnvalue))
  (|CallParentFunction)
  (Utilities|FlowControl|Delay 0.2)
  (Utilities|FlowControl|Sequence
    (:then_0
      (bind _returnvalue_3 (Actor|GetActorOfClass "/Game/Blueprint/ManagerActor/BP_GameFlowManager.BP_GameFlowManager_C"))
      (Utilities|IsValid _returnvalue_3
        (:Is%20Valid
          (Variables|Default|SetTutoMng _returnvalue_3))))
    (:then_1
      (Utilities|IsValid _returnvalue_2
        (:Is%20Valid
          (bind _assr_hud (Utilities|Casting|CastToSR_HUD _returnvalue_2))
          (for _array_element (Variables|/Script/Subject_Rem.SRHUD|GetAddedViewportWidgets _assr_hud)
            (bind _aswb_game_caption (Utilities|Casting|CastToWB_GameCaption _array_element))
            (Utilities|IsValid (Variables|/Game/Blueprint/UI/HUD/GameCaption/WB_GameCaption.WB_GameCaption_C|GetCaption (Class|SRHUD|GetWidgetbyClass _assr_hud "/Game/Blueprint/UI/HUD/GameCaption/WB_GameCaption.WB_GameCaption_C" true))
              (:Is%20Valid
                (EventDispatchers|BindEventtoTypeWriterEndAnimFinished (Variables|/Game/Blueprint/UI/HUD/GameCaption/WB_GameCaption.WB_GameCaption_C|GetCaption _aswb_game_caption) (delegate EventOnCaptionFinished))
                (EventDispatchers|BindEventtoOnTypeWriterStart (Variables|/Game/Blueprint/UI/HUD/GameCaption/WB_GameCaption.WB_GameCaption_C|GetCaption _aswb_game_caption) (EventDispatchers|CreateEvent :!event Custom|OnCaptionStart))))))))))

(event Collision|EventActorBeginOverlap
  (params (OtherActor :type Actor%20Object%20Reference)))

(event EventTick
  (params (DeltaSeconds :type Float%20%28single-precision%29)))

(event EventOnCaptionFinished
  (params (RowName :type Name :default "None"))
  (|CallParentFunction RowName)
  (Default|CallCaptionTypewriterCompletedDelgate RowName)
  (Development|PrintString (Utilities|String|Append "CaptionFinish" (Utilities|String|ToString(Name) RowName))))

(fn ConstructionScript)