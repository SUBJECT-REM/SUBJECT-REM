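; BP_ActivateManager is a manager actor that makes interactable actors visible by key.
; Its construction script gathers every BP_InteractableActor in the level into a map keyed by each actor's DataTableHandler row name.
; ActivateActor looks up the given key in that map, unhides the matching actor and prints a debug message.
; The map is built only at construction, as the event graph has no active logic.
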(event EventBeginPlay)

(event Collision|EventActorBeginOverlap
  (params (OtherActor :type Actor%20Object%20Reference)))

(fn ConstructionScript
  (CallFunction|FindActivateableActor))

(fn FindActivateableActor
  (bind _outactors (Actor|GetAllActorsOfClass "/Game/Blueprint/Interactable/BP_InteractableActor.BP_InteractableActor_C"))
  (for _array_element _outactors
    (Utilities|IsValid _array_element
      (:Is%20Valid
        (Utilities|Map|Add (Variables|Default|GetNewVar) (.RowName (Utilities|Struct|BreakDataTableRowHandle (Variables|/Game/Blueprint/Interactable/BP_InteractableActor.BP_InteractableActor_C|GetDataTableHandler _array_element))) _array_element)))))

(fn ActivateActor
  (params (NewParam :type Name))
  (bind _newvar (Variables|Default|GetNewVar))
  (bind (_value _returnvalue) (Utilities|Map|Find _newvar NewParam))
  (if _returnvalue
    (Rendering|SetActorHiddenInGame _value false)
    (Development|PrintString "actor visible")))